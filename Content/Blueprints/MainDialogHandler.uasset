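; Dialog handler that builds a Conversation actor from a parsed script text file, loading "ScriptA" on BeginPlay.
; CreateConversation reads item interrupt pairs from the first line, then splits later lines at brace markers into important and non-important sections.
; Important sections carry counter results parsed from their closing line.
; ConvertStringToDialogLine parses speaker, text and duration but is never called here, so sections receive empty line arrays.
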(event `self.ReceiveBeginPlay`
  (`self.CreateConversation` "ScriptA"))

(fn `ConvertStringToDialogLine`
  (params (LineFromFile :type String))
  (returns (Results :type "/Game/Blueprints/DialogLine Structure"))
  (bind _returnvalue (`KismetStringLibrary.ParseIntoArray` LineFromFile ":"))
  (bind _output (`|GetArrayItem` _returnvalue))
  (bind _output_2 (`|GetArrayItem` _returnvalue 1))
  (return (make `/Game/Blueprints/DialogLine` (`KismetStringLibrary.GetSubstring` _output 1 (- (`KismetStringLibrary.Len` _output) 2)) (`KismetStringLibrary.GetSubstring` _output_2 1 (- (`KismetStringLibrary.Len` _output_2) 2)) (`KismetStringLibrary.Conv_StringToDouble` (`|GetArrayItem` _returnvalue 2)))))

(fn `CreateConversation`
  (params (FileName :type String))
  (locals (InImportant :type Boolean :default false) (CurrentLines :type "Array of /Game/Blueprints/DialogLine Structure") (CurrentResults :type "Map of String to Integer") (Conversation :type "/Game/Blueprints/Conversation Object Reference"))
  (bind _returnvalue (`KismetStringLibrary.ParseIntoArray` (`KismetStringLibrary.TrimTrailing` (`KismetStringLibrary.Trim` (`ReadFileBlueprintFunctionLibrary.FileLoadString` (`KismetStringLibrary.Concat_StrStr` (`KismetStringLibrary.Concat_StrStr` "/Content/Writing/Script" FileName) "Parsed.txt")))) "<br>"))
  (bind _returnvalue_2 (`|SpawnActorFromClass` "/Game/Blueprints/Conversation.Conversation_C" (`self.GetTransform`) "AlwaysSpawn" "OverrideRootScale" null null))
  (set `local.Conversation` _returnvalue_2)
  ;[1 1 1] Adding Item Interrupt Data to Conversation
  (for _array_element (`KismetStringLibrary.ParseIntoArray` (`|GetArrayItem` (`KismetStringLibrary.ParseIntoArray` (`|GetArrayItem` _returnvalue) ":") 1) "|")
    (bind _returnvalue_3 (`KismetStringLibrary.ParseIntoArray` _array_element "-"))
    (`/Game/Blueprints/Conversation.Add Interrupt` (`local.Conversation`) (`|GetArrayItem` _returnvalue_3) (`|GetArrayItem` _returnvalue_3 1)))
  (set `local.InImportant` true)
  (set `local.CurrentLines` (`|MakeArray`))
  (for (_array_element_2 _array_index) _returnvalue
    ;[1 1 1] Make sure we are not on the first line, and that the line doesn't start with n
    (if (!= _array_index 0)
      (if (not (`KismetStringLibrary.StartsWith` _array_element_2 "n"))
        ;[1 1 1] Check if we have been parsing an important piece of dialog
        (if (`local.InImportant`)
          ;[1 1 1] Check if important dialog is finished
          (if (`KismetStringLibrary.StartsWith` _array_element_2 "}")
            ;[1 1 1] Add the counter increment/decrement information to the ConversationSection
            (set `local.CurrentResults` (`|MakeMap`))
            (for _array_element_3 (`KismetStringLibrary.ParseIntoArray` (`KismetStringLibrary.GetSubstring` _array_element_2 1 (`KismetStringLibrary.Len` _array_element_2)) "|")
              (bind _returnvalue_4 (`KismetStringLibrary.ParseIntoArray` _array_element_3 ","))
              (`BlueprintMapLibrary.Map_Add` (`local.CurrentResults`) (`|GetArrayItem` _returnvalue_4) (`KismetStringLibrary.Conv_StringToInt` (`|GetArrayItem` _returnvalue_4 1))))
            ;[1 1 1] This conversation section is over, add it to the conversation.
            (`/Game/Blueprints/Conversation.AddConversationSegment` (`local.Conversation`) (make `/Game/Blueprints/ConversationSection` true (`local.CurrentLines`) (`local.CurrentResults`)))
            (set `local.InImportant` false))
          (elif (`KismetStringLibrary.StartsWith` _array_element_2 "{")
            (bind _output_get (set `local.CurrentResults` (`|MakeMap`)))
            (`/Game/Blueprints/Conversation.AddConversationSegment` (`local.Conversation`) (make `/Game/Blueprints/ConversationSection` false (`local.CurrentLines`) _output_get))
            (set `local.InImportant` true)))))))

(fn `UserConstructionScript`)