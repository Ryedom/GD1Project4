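; Conversation Blueprint that stores the data for one dialogue: its segments, keyed interrupts and follow-up conversations.
; Setters and getters fill and query these, with segments fetched by index and interrupts by key.
; Segments hold speaker lines with durations and optional killed conversations, plus an importance flag and a results map.
; PrintConversation dumps the whole structure for debugging.
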(fn `Add Interrupt`
  (params (Key :type String) (Value :type "/Game/Blueprints/ItemInterruptConversationArray Structure"))
  (`BlueprintMapLibrary.Map_Add` (`self.Interrupts`) Key Value))

(fn `AddConversationSegment`
  (params (Section :type "/Game/Blueprints/ConversationSection Structure"))
  (`KismetArrayLibrary.Array_Add` (`self.ConversationSections`) Section))

(fn `GetConversationSection`
  (params (index :type Integer))
  (returns (section :type "/Game/Blueprints/ConversationSection Structure"))
  (return (`|GetArrayItem` (`self.ConversationSections`) index)))

(fn `GetInterrupt`
  (params (Key :type String))
  (returns (Value :type "/Game/Blueprints/ItemInterruptConversationArray Structure") (Found :type Boolean))
  (bind (_value _returnvalue) (`BlueprintMapLibrary.Map_Find` (`self.Interrupts`) Key))
  (return _value _returnvalue))

(fn `PrintConversation`
  (`KismetSystemLibrary.PrintString` "Interrupts:" false)
  ;[1 1 1] Printing Interrupts
  (bind _keys (`BlueprintMapLibrary.Map_Keys` (`self.Interrupts`)))
  (for _array_element _keys
    (`KismetSystemLibrary.PrintString` (`KismetStringLibrary.Concat_StrStr` _array_element ":" (`KismetStringLibrary.JoinStringArray` (`.Conversations_3_1315FE62884DF7D7C110D88966DF7EB9` (break `/Game/Blueprints/ItemInterruptConversationArray` (`BlueprintMapLibrary.Map_Find` (`self.Interrupts`) _array_element))) ",")) false))
  (`KismetSystemLibrary.PrintString` "Conversation Segments:" false)
  (for _array_element_2 (`self.ConversationSections`)
    (bind (_important _lines _results) (break `/Game/Blueprints/ConversationSection` _array_element_2))
    (if _important
      (`KismetSystemLibrary.PrintString` "Important" false))
    ;[1 1 1] print each line of dialog
    (for _array_element_3 _lines
      (bind (_speaker _text _duration _kills _killedconversations) (break `/Game/Blueprints/DialogLine` _array_element_3))
      (`KismetSystemLibrary.PrintString` (`KismetStringLibrary.Concat_StrStr` _speaker ":" _text "(" (`KismetStringLibrary.Conv_DoubleToString` _duration) ")") false)
      (if _kills
        (`KismetSystemLibrary.PrintString` "Kills:" false)
        (for _array_element_4 _killedconversations
          (`KismetSystemLibrary.PrintString` _array_element_4 false))))
    (`KismetSystemLibrary.PrintString` "Results:" false)
    (bind _keys_2 (`BlueprintMapLibrary.Map_Keys` _results))
    (for _array_element_5 _keys_2
      (`KismetSystemLibrary.PrintString` (`KismetStringLibrary.Concat_StrStr` _array_element_5 ":" (`KismetStringLibrary.Conv_IntToString` (`BlueprintMapLibrary.Map_Find` _results _array_element_5))) false))
    (`KismetSystemLibrary.PrintString` "End Section" false))
  (`KismetSystemLibrary.PrintString` "Next  Conversations:" false)
  (for _array_element_6 (`self.NextConversation`)
    (`KismetSystemLibrary.PrintString` _array_element_6 false)))

(fn `SetNextConversation`
  (params (NextConversation :type "Array of String"))
  (set `self.NextConversation` NextConversation))

(fn `UserConstructionScript`)